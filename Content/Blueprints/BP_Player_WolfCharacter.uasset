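; Player-controlled wolf character Blueprint that acts as the leader of a wolf pack.
; It extends the parent's Run and Howl events to notify WolfPackComponent that the leader is dynamic or howling.
; BeginPlay also starts a 2D forest ambience sound, while Tick, overlap and construction add no logic of their own.
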(event EventBeginPlay
  (|CallParentFunction)
  (Audio|PlaySound2D "/Game/Audio/201585-Forest_Ambience_Pine_Birch_Summer_Day_Light_Heavy_Wind_Gust_Leaves_Rustle_Distant_Bird_Tweet_Chirp.201585-Forest_Ambience_Pine_Birch_Summer_Day_Light_Heavy_Wind_Gust_Leaves_Rustle_Distant_Bird_Tweet_Chirp" 0.8 1.0 0.0 0 0))

(event Collision|EventActorBeginOverlap
  (params (OtherActor :type Actor%20Object%20Reference))
  (|CallParentFunction OtherActor) ; This node is disabled and will not be called.\nDrag off pins to build functionality.
)

(event EventTick
  (params (DeltaSeconds :type Float%20%28single-precision%29))
  (|CallParentFunction DeltaSeconds) ; This node is disabled and will not be called.\nDrag off pins to build functionality.
)

(event EventRun
  (|CallParentFunction)
  (Default|LeaderIsDynamic (Variables|Default|GetWolf%20Pack%20Component)))

(event EventHowl
  (|CallParentFunction)
  (Default|LeaderIsHowling (Variables|Default|GetWolf%20Pack%20Component)))

(fn ConstructionScript
  (|CallParentFunction))