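; BP_WolfCharacter_PackMember is a pack-member wolf character that follows a parent class and adds variation between individuals.
; On BeginPlay it randomly shrinks the mesh scale per axis and lowers walking and running speeds within set ranges, then calls the parent BeginPlay.
; SetWolfPackLeader forwards the given alpha wolf to the AI controller as pack leader.
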(event EventBeginPlay
  (bind _returnvalue (Math|Random|RandomFloatinRange 0.75 0.9))
  (Transformation|SetWorldScale3D (Variables|Character|GetMesh) (Math|Vector|MakeVector _returnvalue _returnvalue _returnvalue))
  (Variables|Default|SetWalking%20Speed (Math|Random|RandomFloatinRange (- (Variables|Default|GetWalking%20Speed) 5e+01) (Variables|Default|GetWalking%20Speed)))
  (Variables|Default|SetRunning%20Speed (Math|Random|RandomFloatinRange (- (Variables|Default|GetRunning%20Speed) 1e+02) (Variables|Default|GetRunning%20Speed)))
  (|CallParentFunction))

(event Collision|EventActorBeginOverlap
  (params (OtherActor :type Actor%20Object%20Reference))
  (|CallParentFunction OtherActor) ; This node is disabled and will not be called.\nDrag off pins to build functionality.
)

(event EventTick
  (params (DeltaSeconds :type Float%20%28single-precision%29))
  (|CallParentFunction DeltaSeconds) ; This node is disabled and will not be called.\nDrag off pins to build functionality.
)

(fn ConstructionScript
  (|CallParentFunction))

(fn SetWolfPackLeader
  (params (Alpha%20Wolf :type BP%20Player%20Wolf%20Character%20Object%20Reference))
  (Default|SetWolfPackLeader (Variables|Default|GetAI%20Controller%20Ref) Alpha%20Wolf))