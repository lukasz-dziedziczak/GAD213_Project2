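; Actor component on the player wolf character that spawns and leads an AI wolf pack.
; Each tick it spawns one wolf at a random navigable point within the follow radius until the pack size is reached, assigning the player as its leader.
; Leader howl and dynamic-state changes are relayed to every pack member through its AI controller.
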(event Custom|Spawn
  (bind _wolf_prefab (Variables|Default|GetWolf%20Prefab)
    (:then
      (bind _location (CallFunction|LocationinFollowRadius))
      (bind _returnvalue (Game|SpawnActorfromClass _wolf_prefab (Math|Transform|MakeTransform _location "0, 0, 0" "1.000000,1.000000,1.000000") "AdjustIfPossibleButAlwaysSpawn" "MultiplyWithRoot" 0 0))
      (Utilities|IsValid _returnvalue
        (:Is%20Valid
          (Utilities|Array|Add (Variables|Default|GetWolves) _returnvalue)
          (Default|SetWolfPackLeader _returnvalue (Variables|Default|GetAlpha%20Wolf)))))
    (:else)))

(event Custom|Spawn%20Wolf%20Pack
  (if (< (Utilities|Array|Length (Variables|Default|GetWolves)) (Variables|Default|GetPack%20Size))
    (CallFunction|Spawn)))

(event Custom|Leader%20Is%20Howling
  (for _array_element (Variables|Default|GetWolves)
    (Default|LeaderIsHowling (Variables|/Game/Blueprints/BP_AnimalCharacter.BP_AnimalCharacter_C|GetAI%20Controller%20Ref _array_element))))

(event Custom|Leader%20Is%20Dynamic
  (for _array_element (Variables|Default|GetWolves)
    (Default|LeaderGoneDynamic (Variables|/Game/Blueprints/BP_AnimalCharacter.BP_AnimalCharacter_C|GetAI%20Controller%20Ref _array_element))))

(event EventTick
  (params (DeltaSeconds :type Float%20%28single-precision%29))
  (CallFunction|SpawnWolfPack))

(event EventBeginPlay
  (bind _asbp_player_wolf_character (Utilities|Casting|CastToBP_Player_WolfCharacter (Components|GetOwner)))
  (Variables|Default|SetAlpha%20Wolf _asbp_player_wolf_character))

(fn LocationinFollowRadius
  (bind _randomlocation (Class|NavigationSystemV1|GetRandomLocationinNavigableRadius (Transformation|GetActorLocation (Components|GetOwner)) (Variables|Default|GetFollow%20Radius) 0 0))
  (return _randomlocation))

(fn SetLeaderIsDynamic
  (params (Is%20Dynamic :type Boolean))
  (for _array_element (Variables|Default|GetWolves)
    (Variables|/Game/AI/BP_AI_Controller.BP_AI_Controller_C|SetLeader%20Is%20Dynamic (Variables|/Game/Blueprints/BP_AnimalCharacter.BP_AnimalCharacter_C|GetAI%20Controller%20Ref _array_element) Is%20Dynamic)))