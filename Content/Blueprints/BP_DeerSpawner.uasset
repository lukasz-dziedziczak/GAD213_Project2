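; Spawner actor that keeps a population of deer in a spherical area, pausing spawns while any wolf is inside it.
; Tick spawns a random Deer or Doe at a reachable navmesh point in the sphere until DeerList reaches NumberToSpawn.
; Sphere overlaps track wolves in WolfList and notify its own deer when they leave or return to the area.
; Each spawned deer holds a reference to the spawner, and RemoveDeer takes one off the list.
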(event OnComponentBeginOverlap(Sphere)
  (params (OverlappedComponent :type Primitive%20Component%20Object%20Reference) (OtherActor :type Actor%20Object%20Reference) (OtherComp :type Primitive%20Component%20Object%20Reference) (OtherBodyIndex :type Integer) (bFromSweep :type Boolean) (SweepResult :type Hit%20Result%20Structure%20%28by%20ref%29))
  (Utilities|FlowControl|Sequence
    (:then_0
      (bind _asbp_deer_character (Utilities|Casting|CastToBP_DeerCharacter OtherActor))
      (if (Utilities|Array|ContainsItem (Variables|Default|GetDeer%20List) _asbp_deer_character)
        (Default|ReturnedtoSpawnArea _asbp_deer_character)))
    (:then_1
      (bind _asbp_wolf_character (Utilities|Casting|CastToBP_WolfCharacter OtherActor))
      (Utilities|Array|Add (Variables|Default|GetWolf%20List) _asbp_wolf_character))))

(event OnComponentEndOverlap(Sphere)
  (params (OverlappedComponent :type Primitive%20Component%20Object%20Reference) (OtherActor :type Actor%20Object%20Reference) (OtherComp :type Primitive%20Component%20Object%20Reference) (OtherBodyIndex :type Integer))
  (Utilities|FlowControl|Sequence
    (:then_0
      (bind _asbp_deer_character (Utilities|Casting|CastToBP_DeerCharacter OtherActor))
      (if (Utilities|Array|ContainsItem (Variables|Default|GetDeer%20List) _asbp_deer_character)
        (Default|LeftSpawnedArea _asbp_deer_character)))
    (:then_1
      (bind _asbp_wolf_character (Utilities|Casting|CastToBP_WolfCharacter OtherActor))
      (Utilities|Array|RemoveItem (Variables|Default|GetWolf%20List) _asbp_wolf_character))))

(event Custom|Spawn
  (bind _randomlocation (CallFunction|RandomSpotinArea))
  (if (Math|Random|RandomBool)
    (bind _returnvalue (Game|SpawnActorfromClass (Variables|Default|GetDeer) (Math|Transform|MakeTransform _randomlocation "0, 0, 0" "1.000000,1.000000,1.000000") "AdjustIfPossibleButDontSpawnIfColliding" "MultiplyWithRoot" 0 0))
    (Utilities|IsValid _returnvalue
      (:Is%20Valid
        (Variables|/Game/Blueprints/BP_AnimalCharacter.BP_AnimalCharacter_C|SetDeer%20Spawner _returnvalue self)
        (Utilities|Array|Add (Variables|Default|GetDeer%20List) _returnvalue)))
    (else
      (bind _returnvalue_2 (Game|SpawnActorfromClass (Variables|Default|GetDoe) (Math|Transform|MakeTransform _randomlocation "0, 0, 0" "1.000000,1.000000,1.000000") "AdjustIfPossibleButDontSpawnIfColliding" "MultiplyWithRoot" 0 0))
      (Utilities|IsValid _returnvalue_2
        (:Is%20Valid
          (Variables|/Game/Blueprints/BP_AnimalCharacter.BP_AnimalCharacter_C|SetDeer%20Spawner _returnvalue_2 self)
          (Utilities|Array|Add (Variables|Default|GetDeer%20List) _returnvalue_2))))))

(event EventTick
  (params (DeltaSeconds :type Float%20%28single-precision%29))
  (if (and (< (Utilities|Array|Length (Variables|Default|GetDeer%20List)) (Variables|Default|GetNumberToSpawn)) (== (Utilities|Array|Length (Variables|Default|GetWolf%20List)) 0))
    (CallFunction|Spawn)))

(fn ConstructionScript)

(fn RemoveDeer
  (params (Deer :type BP%20Deer%20Character%20Object%20Reference))
  (Utilities|Array|RemoveItem (Variables|Default|GetDeer%20List) Deer))

(fn RandomSpotinArea
  (return (.RandomLocation (AI|Navigation|GetRandomReachablePointinRadius (Transformation|GetActorLocation) (Variables|/Script/Engine.SphereComponent|GetSphereRadius (Variables|Default|GetSphere)) 0 0))))