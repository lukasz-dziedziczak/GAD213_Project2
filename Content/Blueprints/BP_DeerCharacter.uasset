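; Deer character Blueprint that links an AI-controlled deer to the spawn area of its DeerSpawner.
; Events for leaving and returning to that area are relayed to BP_AI_Controller, and returning also calls Walk.
; LocationInSpawnArea returns a random spot from the spawner when that reference is valid.
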(event Custom|Returned%20to%20Spawn%20Area
  (bind _asbp_ai_controller (Utilities|Casting|CastToBP_AI_Controller (Pawn|GetController)))
  (Default|ReturnedtoSpawnArea _asbp_ai_controller)
  (CallFunction|Walk))

(event Custom|Left%20Spawned%20Area
  (bind _asbp_ai_controller (Utilities|Casting|CastToBP_AI_Controller (Pawn|GetController))
    (:then
      (Default|LeftSpawnArea _asbp_ai_controller))
    (:CastFailed
      (Development|PrintString "Did not find AI controller"))))

(event EventBeginPlay
  (|CallParentFunction) ; This node is disabled and will not be called.\nDrag off pins to build functionality.
)

(event Collision|EventActorBeginOverlap
  (params (OtherActor :type Actor%20Object%20Reference))
  (|CallParentFunction OtherActor) ; This node is disabled and will not be called.\nDrag off pins to build functionality.
)

(event EventTick
  (params (DeltaSeconds :type Float%20%28single-precision%29))
  (|CallParentFunction DeltaSeconds) ; This node is disabled and will not be called.\nDrag off pins to build functionality.
)

(fn ConstructionScript
  (|CallParentFunction))

(fn LocationinSpawnArea
  (bind _deer_spawner (Variables|Default|GetDeer%20Spawner)
    (:then
      (bind _randomlocation (Default|RandomSpotinArea _deer_spawner))
      (return _randomlocation))
    (:else)))