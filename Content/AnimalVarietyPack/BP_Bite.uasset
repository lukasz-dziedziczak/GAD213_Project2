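; Bite hitbox for the animal pack that kills animals inside its Sphere when Bite is triggered.
; Sphere begin and end overlap events maintain the OverlapActors list, which Bite loops over, casting to BP_AnimalBase and calling Death.
; BeginPlay caches the Sphere's owner as Animal, but Bite does not check against it.
; An older IsBiting path with an owner check and debug print is left disconnected.
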(event OnComponentBeginOverlap(Sphere)
  (params (OverlappedComponent :type Primitive%20Component%20Object%20Reference) (OtherActor :type Actor%20Object%20Reference) (OtherComp :type Primitive%20Component%20Object%20Reference) (OtherBodyIndex :type Integer) (bFromSweep :type Boolean) (SweepResult :type Hit%20Result%20Structure%20%28by%20ref%29))
  (Utilities|Array|Add (Variables|Default|GetOverlap%20Actors) OtherActor))

(event OnComponentEndOverlap(Sphere)
  (params (OverlappedComponent :type Primitive%20Component%20Object%20Reference) (OtherActor :type Actor%20Object%20Reference) (OtherComp :type Primitive%20Component%20Object%20Reference) (OtherBodyIndex :type Integer))
  (Utilities|Array|RemoveItem (Variables|Default|GetOverlap%20Actors) OtherActor))

(event Custom|Bite
  (for _array_element (Variables|Default|GetOverlap%20Actors)
    (bind _asbp_animal_base (Utilities|Casting|CastToBP_AnimalBase _array_element))
    (Default|Death _asbp_animal_base)))

(event EventBeginPlay
  (bind _asbp_animal_base (Utilities|Casting|CastToBP_AnimalBase (Components|GetOwner (Variables|Default|GetSphere))))
  (Variables|Default|SetAnimal _asbp_animal_base))

(fn ConstructionScript)