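; Playable animal character with Enhanced Input for looking, camera-relative forward/back movement, walk/run speed switching and a bite attack.
; On BeginPlay it adds the mapping context and attaches a spawned BP_Bite actor to the Mouth socket.
; Attacking plays a montage and blocks movement input until completion; Anim_BiteEvent triggers the mouth actor's bite.
; Death clears IsAlive, zeroes walk speed and destroys the actor after a delay.
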(event Custom|Bite
  (bind _bite_montage (Variables|Default|GetBite%20Montage)
    (:then
      (if (not (Variables|Default|GetIs%20Attacking))
        (Animation|Montage|PlayMontage (Variables|Character|GetMesh) _bite_montage
          (:then
            (Variables|Default|SetIs%20Attacking true))
          (:OnCompleted
            (Variables|Default|SetIs%20Attacking false)))))
    (:else
      (Development|PrintString "Bite Montage Invalid"))))

(event Custom|Death
  (Development|PrintString (Utilities|String|Append (Utilities|GetDisplayName self) " died"))
  (Variables|Default|SetIs%20Alive false)
  (Variables|/Script/Engine.CharacterMovementComponent|SetMaxWalkSpeed (Variables|Character|GetCharacterMovement) 0.0)
  (Utilities|FlowControl|Delay 1e+01)
  (Actor|DestroyActor))

(event Custom|Run
  (Variables|/Script/Engine.CharacterMovementComponent|SetMaxWalkSpeed (Variables|Character|GetCharacterMovement) (Variables|Default|GetRunning%20Speed)))

(event Custom|Anim_BiteEvent
  (Default|Bite (Variables|Default|GetMouth%20Bite)))

(event Custom|Walk
  (Variables|/Script/Engine.CharacterMovementComponent|SetMaxWalkSpeed (Variables|Character|GetCharacterMovement) (Variables|Default|GetWalking%20Speed)))

(event Input|EnhancedActionEvents|EnhancedInputActionIA_Move
  (params (ActionValue :type Vector%202D%20Structure) (ElapsedSeconds :type Float%20%28double-precision%29) (TriggeredSeconds :type Float%20%28double-precision%29) (InputAction :type Input%20Action%20Object%20Reference :default "/Game/Input/IA_Move.IA_Move"))
  (bind _camera (Variables|Default|GetCamera))
  (bind _returnvalue (Transformation|GetWorldRotation _camera))
  (bind _returnvalue_2 (Math|Vector|GetForwardVector _returnvalue))
  ;[1 1 1] Movement
  (if (not (Variables|Default|GetIs%20Attacking))
    (Pawn|Input|AddMovementInput (Math|Vector|MakeVector (.x _returnvalue_2) (.y _returnvalue_2) (.z (Transformation|GetActorForwardVector))) (.y ActionValue) false)))

(event Input|EnhancedActionEvents|EnhancedInputActionIA_Look
  (params (ActionValue :type Vector%202D%20Structure) (ElapsedSeconds :type Float%20%28double-precision%29) (TriggeredSeconds :type Float%20%28double-precision%29) (InputAction :type Input%20Action%20Object%20Reference :default "/Game/Input/IA_Look.IA_Look"))
  ;[1 1 1] Look
  (Pawn|Input|AddControllerYawInput (.x ActionValue))
  (Pawn|Input|AddControllerPitchInput (.y ActionValue)))

(event Input|EnhancedActionEvents|EnhancedInputActionIA_Run
  (params (ActionValue :type Boolean) (ElapsedSeconds :type Float%20%28double-precision%29) (TriggeredSeconds :type Float%20%28double-precision%29) (InputAction :type Input%20Action%20Object%20Reference :default "/Game/Input/IA_Run.IA_Run"))
  (:Started
    (CallFunction|Run))
  (:Completed
    (CallFunction|Walk)))

(event Input|EnhancedActionEvents|EnhancedInputActionIA_Attack
  (params (ActionValue :type Boolean) (ElapsedSeconds :type Float%20%28double-precision%29) (TriggeredSeconds :type Float%20%28double-precision%29) (InputAction :type Input%20Action%20Object%20Reference :default "/Game/Input/IA_Attack.IA_Attack"))
  (CallFunction|Bite))

(event EventBeginPlay
  (bind _asbp_player_controler (Utilities|Casting|CastToBP_PlayerControler (Game|GetPlayerController 0)))
  (Utilities|IsValid (PlayerController|LocalPlayerSubsystems|GetEnhancedInputLocalPlayerSubsystem _asbp_player_controler)
    (:Is%20Valid
      (Input|AddMappingContext (PlayerController|LocalPlayerSubsystems|GetEnhancedInputLocalPlayerSubsystem _asbp_player_controler) "/Game/Input/InputMappingContext.InputMappingContext" 0 "(bIgnoreAllPressedKeysUntilRelease=True,bForceImmediately=False,bNotifyUserSettings=False)")
      (CallFunction|Walk)
      (bind _returnvalue (Game|SpawnActorfromClass "/Game/AnimalVarietyPack/BP_Bite.BP_Bite_C" (Transformation|GetActorTransform) "Undefined" "MultiplyWithRoot" 0 0))
      (bind _output_get (Variables|Default|SetMouth%20Bite _returnvalue))
      (Transformation|AttachComponentToComponent _output_get (Variables|Character|GetMesh) (Utilities|Name|MakeLiteralName "Mouth") "SnapToTarget" "SnapToTarget" "KeepRelative" true)
      (Actor|SetOwner _output_get self))))

(fn ConstructionScript)

(fn IsWalking?
  (return (== (Variables|/Script/Engine.CharacterMovementComponent|GetMaxWalkSpeed (Variables|Character|GetCharacterMovement)) (Variables|Default|GetWalking%20Speed))))