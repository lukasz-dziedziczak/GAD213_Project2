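; AI controller for wolf and deer animals that runs a species-specific behavior tree on possession.
; Hearing lets wolves target living deer while their pack leader is dynamic and lets deer register wolf predators; the sight branch is hard-disabled.
; Tick flags the animal's death and clears dead targets.
; Events and functions feed pack leader, howl and spawn-area state to the Blackboard and supply follow locations near the leader.
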(event OnTargetPerceptionUpdated(AIPerception)
  (params (Actor :type Actor%20Object%20Reference) (Stimulus :type AI%20Stimulus%20Structure))
  ;[1 1 1] On Perception Updated
  (CallFunction|SightDetection Actor Stimulus)
  (CallFunction|HearingDetection Actor Stimulus))

(event Custom|Death
  ;[1 1 1] Death
  (AI|Components|Blackboard|SetValueasBool (AI|GetBlackboard 0) (Utilities|Name|MakeLiteralName "IsAlive") false))

(event Custom|Clear%20Predator
  ;[1 1 1] Clear Predator
  (AI|Components|Blackboard|SetValueasObject (AI|GetBlackboard 0) (Utilities|Name|MakeLiteralName "Predator") 0)
  (Variables|Default|SetPredator 0))

(event Custom|Left%20Spawn%20Area
  ;[1 1 1] Left Spawning Area
  (AI|Components|Blackboard|SetValueasBool (AI|GetBlackboard 0) (Utilities|Name|MakeLiteralName "OutSideSpawnArea") true))

(event Custom|Returned%20to%20Spawn%20Area
  ;[1 1 1] Returned to Spawning Area
  (AI|Components|Blackboard|SetValueasBool (AI|GetBlackboard 0) (Utilities|Name|MakeLiteralName "OutSideSpawnArea") false))

(event Custom|Leader%20Is%20Howling
  ;[1 1 1] Leader is Howling
  (Variables|Default|SetLeader%20Is%20Dynamic false)
  (AI|Components|Blackboard|SetValueasObject (AI|GetBlackboard 0) (Utilities|Name|MakeLiteralName "Target") 0)
  (Variables|Default|SetTarget%20Actor 0)
  (AI|Components|Blackboard|SetValueasBool (AI|GetBlackboard 0) (Utilities|Name|MakeLiteralName "LeaderIsDynamic") false))

(event Custom|Leader%20gone%20dynamic
  ;[1 1 1] Leader gone Dynamic
  (Variables|Default|SetLeader%20Is%20Dynamic true)
  (AI|Components|Blackboard|SetValueasBool (AI|GetBlackboard 0) (Utilities|Name|MakeLiteralName "LeaderIsDynamic") true))

(event EventBeginPlay
  ;[1 1 1] On Posses (Sorta like Begin Play)
)

(event EventTick
  (params (DeltaSeconds :type Float%20%28single-precision%29))
  ;[1 1 1] Tick
  (Utilities|FlowControl|Sequence
    (:then_0
      (bind _animal (Variables|Default|GetAnimal)
        (:then
          (if (not (Variables|/Game/Blueprints/BP_AnimalCharacter.BP_AnimalCharacter_C|GetIs%20Alive _animal))
            (if (ScalableFloat|GetValueasBool (AI|GetBlackboard 0) (Utilities|Name|MakeLiteralName "IsAlive"))
              (CallFunction|Death))))
        (:else)))
    (:then_1
      (bind _target_actor (Variables|Default|GetTarget%20Actor)
        (:then
          (if (not (Variables|/Game/Blueprints/BP_AnimalCharacter.BP_AnimalCharacter_C|GetIs%20Alive _target_actor))
            (AI|Components|Blackboard|SetValueasObject (AI|GetBlackboard 0) (Utilities|Name|MakeLiteralName "Target") 0)
            (Variables|Default|SetTarget%20Actor 0)
            (bind _animal_2 (Variables|Default|GetAnimal)
              (:then
                (Default|Walk _animal_2))
              (:else))))
        (:else)))))

(event EventPossess
  (params (PossessedPawn :type Pawn%20Object%20Reference))
  ;[1 1 1] On Posses (Sorta like Begin Play)
  (Utilities|FlowControl|Sequence
    (:then_0
      (bind _asbp_animal_character (Utilities|Casting|CastToBP_AnimalCharacter (Pawn|GetControlledPawn)))
      (bind _output_get (Variables|Default|SetAnimal _asbp_animal_character))
      (Utilities|FlowControl|Sequence
        (:then_0
          (bind _asbp_deer_character (Utilities|Casting|CastToBP_DeerCharacter _output_get))
          (Variables|Default|SetDeer _asbp_deer_character)
          (AI|RunBehaviorTree "/Game/AI/BT_Deer.BT_Deer"))
        (:then_1
          (bind _asbp_wolf_character (Utilities|Casting|CastToBP_WolfCharacter _output_get))
          (Variables|Default|SetWolf _asbp_wolf_character)
          (AI|RunBehaviorTree "/Game/AI/BT_Wolf.BT_Wolf"))))
    (:then_1
      (bind _animal (Variables|Default|GetAnimal)
        (:then
          (AI|Components|Blackboard|SetValueasBool (AI|GetBlackboard 0) (Utilities|Name|MakeLiteralName "HasWaypoints") (> (Utilities|Array|Length (Variables|/Game/AI/BPC_WaypointSystem.BPC_WaypointSystem_C|GetWaypoint%20List (Variables|/Game/Blueprints/BP_AnimalCharacter.BP_AnimalCharacter_C|GetWaypointSystem _animal))) 0)))
        (:else)))))

(fn ConstructionScript)

(fn SightDetection
  (params (Actor :type Actor%20Object%20Reference) (Stimulus :type AI%20Stimulus%20Structure))
  (bind _returnvalue (Class|AIPerceptionSystem|GetSenseClassforStimulus Stimulus))
  (if (and false (.bSuccessfullySensed (Utilities|Struct|BreakAIStimulus Stimulus)))
    (Utilities|FlowControl|Sequence
      (:then_0
        (Variables|Default|GetTarget%20Actor
          (:then)
          (:else
            (Variables|Default|GetWolf
              (:then
                (bind _asbp_deer_character (Utilities|Casting|CastToBP_DeerCharacter Actor))
                (if (and (Variables|/Game/Blueprints/BP_AnimalCharacter.BP_AnimalCharacter_C|GetIs%20Alive _asbp_deer_character) (Variables|Default|GetLeader%20Is%20Dynamic))
                  (AI|Components|Blackboard|SetValueasObject (AI|GetBlackboard 0) (Utilities|Name|MakeLiteralName "Target") Actor)
                  (Variables|Default|SetTarget%20Actor _asbp_deer_character)))
              (:else)))))
      (:then_1
        (Variables|Default|GetDeer
          (:then
            (Variables|Default|GetPredator
              (:then)
              (:else
                (bind _asbp_wolf_character (Utilities|Casting|CastToBP_WolfCharacter Actor))
                (bind _output_get (Variables|Default|SetPredator _asbp_wolf_character))
                (AI|Components|Blackboard|SetValueasObject (AI|GetBlackboard 0) (Utilities|Name|MakeLiteralName "Predator") _output_get))))
          (:else))))))

(fn HearingDetection
  (params (Actor :type Actor%20Object%20Reference) (Stimulus :type AI%20Stimulus%20Structure))
  (bind _returnvalue (Class|AIPerceptionSystem|GetSenseClassforStimulus Stimulus))
  (if (and (== _returnvalue "/Script/AIModule.AISense_Hearing") (.bSuccessfullySensed (Utilities|Struct|BreakAIStimulus Stimulus)))
    (Utilities|FlowControl|Sequence
      (:then_0
        (Variables|Default|GetTarget%20Actor
          (:then)
          (:else
            (Variables|Default|GetWolf
              (:then
                (bind _asbp_deer_character (Utilities|Casting|CastToBP_DeerCharacter Actor))
                (if (and (Variables|/Game/Blueprints/BP_AnimalCharacter.BP_AnimalCharacter_C|GetIs%20Alive _asbp_deer_character) (Variables|Default|GetLeader%20Is%20Dynamic))
                  (AI|Components|Blackboard|SetValueasObject (AI|GetBlackboard 0) (Utilities|Name|MakeLiteralName "Target") Actor)
                  (Variables|Default|SetTarget%20Actor _asbp_deer_character)))
              (:else)))))
      (:then_1
        (Variables|Default|GetDeer
          (:then
            (Variables|Default|GetPredator
              (:then)
              (:else
                (bind _asbp_wolf_character (Utilities|Casting|CastToBP_WolfCharacter Actor))
                (Variables|Default|SetPredator _asbp_wolf_character)
                (AI|Components|Blackboard|SetValueasObject (AI|GetBlackboard 0) (Utilities|Name|MakeLiteralName "Predator") _asbp_wolf_character))))
          (:else))))))

(fn SetWolfPackLeader
  (params (Alpha%20Wolf :type BP%20Player%20Wolf%20Character%20Object%20Reference))
  (AI|Components|Blackboard|SetValueasObject (Variables|Default|GetBlackboard) (Utilities|Name|MakeLiteralName "Leader") Alpha%20Wolf)
  (Variables|Default|SetLeader Alpha%20Wolf))

(fn GetLocationNearWolfPackLeader
  (bind _leader (Variables|Default|GetLeader)
    (:then
      (bind _location (Default|LocationinFollowRadius (Variables|/Game/Blueprints/BP_Player_WolfCharacter.BP_Player_WolfCharacter_C|GetWolf%20Pack%20Component _leader)))
      (return _location))
    (:else
      (Development|PrintString "Leader not set on Controller"))))